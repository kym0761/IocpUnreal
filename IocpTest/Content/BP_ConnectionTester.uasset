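; BP_ConnectionTester is a Blueprint that drives a game server connection through the TestGameInstance.
; It connects to the server on BeginPlay, processes received packets every Tick, and disconnects on EndPlay.
; Each event casts the game instance to TestGameInstance and delegates the work to its functions, so the Blueprint holds no networking logic of its own.
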(event EventBeginPlay
  (bind _astest_game_instance (Utilities|Casting|CastToTestGameInstance (Game|GetGameInstance)))
  (Class|TestGameInstance|ConnecttoGameServer _astest_game_instance))

(event EventTick
  (params (DeltaSeconds :type Float%20%28single-precision%29))
  (bind _astest_game_instance (Utilities|Casting|CastToTestGameInstance (Game|GetGameInstance)))
  (Class|TestGameInstance|HandleRecvPackets _astest_game_instance))

(event EventEndPlay
  (params (EndPlayReason :type EEndPlayReason%20Enum :default "Destroyed"))
  (bind _astest_game_instance (Utilities|Casting|CastToTestGameInstance (Game|GetGameInstance)))
  (Class|TestGameInstance|DisconnectfromGameServer _astest_game_instance))

(fn ConstructionScript)